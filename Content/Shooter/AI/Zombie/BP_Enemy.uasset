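; BP_Enemy is the zombie enemy character for the shooter, with walk/run speed switching and an overhead health widget that turns toward the player every tick.
; While active, its attack trigger damages an overlapped main character through that character's health component and heals the enemy.
; When its health component reports death, it disables capsule collision, stops AI logic, removes the widget and starts a timer for delayed cleanup.
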(event `self.ReceiveBeginPlay`
  (bind _aswbp_health_enemy (cast `/Game/Shooter/UI/CustomUI/WBP_HealthEnemy` (`WidgetComponent.GetWidget` (`self.Widget`))))
  (set `/Game/Shooter/UI/CustomUI/WBP_HealthEnemy.AiOwner` self _aswbp_health_enemy))

(event `self.Attack Trigger.OnComponentBeginOverlap`
  (params (OverlappedComponent :type "PrimitiveComponent Object Reference") (OtherActor :type "Actor Object Reference") (OtherComp :type "PrimitiveComponent Object Reference") (OtherBodyIndex :type Integer) (bFromSweep :type Boolean) (SweepResult :type "HitResult Structure (by ref)"))
  (if (`self.AttackTriggerActive`)
    (bind _asbp_main_character (cast `/Game/Shooter/Core/BP_MainCharacter` OtherActor))
    (bind _returnvalue (`SMainCharacter.GetHealthComponent` _asbp_main_character))
    (`/Engine/EditorBlueprintResources/StandardMacros.IsValid` _returnvalue
      (:`Is Valid`
        (`SHealthComponent.TakeDamage` _returnvalue (`self.Damage`) self)
        (`SHealthComponent.GainHealth` (`self.BPC_HealthComponent`) (`self.HealingValue`))))))

(event `self.ReceiveTick`
  (params (DeltaSeconds :type "Float (single-precision)"))
  (bind _returnvalue (`GameplayStatics.GetPlayerCharacter` 0))
  (`/Engine/EditorBlueprintResources/StandardMacros.IsValid` (`self.Widget`)
    (:`Is Valid`
      (`/Engine/EditorBlueprintResources/StandardMacros.IsValid` _returnvalue
        (:`Is Valid`
          (`SceneComponent.K2_SetWorldRotation` (`self.Widget`) (`KismetMathLibrary.FindLookAtRotation` (`SceneComponent.K2_GetComponentLocation` (`self.Widget`)) (`self.K2_GetActorLocation` _returnvalue)) false false))))))

(event `self.BPC_HealthComponent.OnDead`
  (`self.Die`))

(fn `DestroySelf`
  (`self.K2_DestroyActor`))

(fn `Die`
  (`PrimitiveComponent.SetCollisionEnabled` (`self.CapsuleComponent`) "NoCollision")
  (`BrainComponent.StopLogic` (`AIController.BrainComponent` (`AIBlueprintHelperLibrary.GetAIController` self)) "I am dead")
  (`ActorComponent.K2_DestroyComponent` (`self.Widget`))
  (`KismetSystemLibrary.K2_SetTimerDelegate` (`|CreateDelegate` :!event `DestroySelf`) (`self.DestroyActorTime`)))

(fn `Update Walk Speed`
  (params (`Is Running` :type Boolean))
  (set `CharacterMovementComponent.MaxWalkSpeed` (`KismetMathLibrary.SelectFloat` (`self.RunSpeed`) (`self.WalkSpeed`) `Is Running`) (`self.CharacterMovement`)))

(fn `UserConstructionScript`)