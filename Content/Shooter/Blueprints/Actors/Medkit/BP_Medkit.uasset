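; BP_Medkit is a shooter pickup that heals a character on interaction.
; Interact checks for an SHealthComponent below max health, then plays a sound, applies HealValue through GainHealth and calls StartReset.
; StartReset hides the actor, disables its collision and starts a looping timer of ResetTime, while Reset restores visibility and collision so the medkit can be reused.
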(event `/Game/Shooter/Interfaces/BPI_Interact.Interact`
  (params (InCharacter :type "Character Object Reference"))
  (bind _returnvalue (`self.GetComponentByClass` InCharacter "/Script/Shooter.SHealthComponent"))
  (`/Engine/EditorBlueprintResources/StandardMacros.IsValid` _returnvalue
    (:`Is Valid`
      (if (!= (`SHealthComponent.GetCurrentHealth` _returnvalue) (`SHealthComponent.GetMaxHealth` _returnvalue))
        (`GameplayStatics.PlaySound2D` "/Game/Shooter/Blueprints/Actors/Medkit/Sounds/Medkit.Medkit" 1.0 1.0 0.0 null null)
        (`SHealthComponent.GainHealth` _returnvalue (`self.HealValue `))
        (`self.StartReset`)))))

(fn `Reset`
  (`self.SetActorHiddenInGame` false)
  (`self.SetActorEnableCollision` true))

(fn `StartReset`
  (`self.SetActorHiddenInGame` true)
  (`self.SetActorEnableCollision` false)
  (`KismetSystemLibrary.K2_SetTimerDelegate` (`|CreateDelegate` :!event `Reset`) (`self.ResetTime`) true))

(fn `UserConstructionScript`)