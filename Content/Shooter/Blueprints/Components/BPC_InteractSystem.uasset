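; Actor component that lets its owning character interact with objects in the world.
; On BeginPlay it caches the owner as a Character, stopping if the cast fails.
; Interact line-traces on the Visibility channel from the character's camera along its forward vector up to InteractDistance.
; A hit actor implementing BPI_Interact receives InteractMessage with the character as argument.
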(event `self.ReceiveBeginPlay`
  (`self.Initialize`))

(fn `Initialize`
  (bind _ascharacter (cast `Character` (`self.GetOwner`)))
  (set `self.OwnerCharacter` _ascharacter))

(fn `Interact`
  (bind _returnvalue (`Actor.GetComponentByClass` (`self.OwnerCharacter`) "/Script/Engine.CameraComponent"))
  (bind _returnvalue_2 (`SceneComponent.K2_GetComponentLocation` _returnvalue))
  (bind (_outhit _returnvalue_3) (`KismetSystemLibrary.LineTraceSingle` _returnvalue_2 (+ _returnvalue_2 (* (`SceneComponent.GetForwardVector` _returnvalue) (`self.InteractDistance`))) "TraceTypeQuery1"))
  (if _returnvalue_3
    (bind (_bblockinghit _binitialoverlap _time _distance _location _impactpoint _normal _impactnormal _physmat _hitactor) (`GameplayStatics.BreakHitResult` _outhit))
    (if (`KismetSystemLibrary.DoesImplementInterface` _hitactor "/Game/Shooter/Interfaces/BPI_Interact.BPI_Interact_C")
      (message `/Game/Shooter/Interfaces/BPI_Interact.Interact` _hitactor (`self.OwnerCharacter`)))))