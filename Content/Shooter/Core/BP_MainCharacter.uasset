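; BP_MainCharacter is the shooter's main character, wiring input and health events to interaction and feedback.
; Pressing E triggers Interact on its BPCInteractSystem component.
; HealthComponent damage events play a 2D sound and add a new WBP_TakeDamage widget to the viewport.
; On death it asks BP_GameInstance to start a level reset, plays a death sound and destroys itself.
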(event `Key|E`
  (params (Key :type "Key Structure"))
  (:`Pressed`
    (`/Game/Shooter/Blueprints/Components/BPC_InteractSystem.Interact` (`self.BPC_InteractSystem`))))

(event `self.HealthComponent.OnDead`
  (`self.Dead`))

(event `self.HealthComponent.OnTakeDamage`
  (`self.TakeDamage`))

(fn `Dead`
  (`/Game/Shooter/Blueprints/BP_GameInstance.StartResetLevel` (cast `/Game/Shooter/Blueprints/BP_GameInstance` (`GameplayStatics.GetGameInstance`) :!pure true))
  (`GameplayStatics.PlaySound2D` "/Game/Shooter/Core/Sounds/Dead.Dead" 1.0 1.0 0.0 null null)
  (`self.K2_DestroyActor`))

(fn `TakeDamage`
  (`GameplayStatics.PlaySound2D` "/Game/Shooter/Core/Sounds/TakeDamage.TakeDamage" 1.0 1.0 0.0 null null)
  (bind _returnvalue (`|CreateWidget` "/Game/Shooter/UI/WBP_TakeDamage.WBP_TakeDamage_C"))
  (`UserWidget.AddToViewport` _returnvalue 0))

(fn `UserConstructionScript`)