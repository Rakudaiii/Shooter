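; Shooter player controller Blueprint that provides helpers for switching between gameplay and UI input.
; Game-only mode hides the cursor and sets the controlled pawn's CharacterMovementComponent back to Walking.
; UI-only mode shows the cursor, focuses the given widget and disables the pawn's movement.
; The event graph is unused.
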(fn `SetInputModeGameOnly`
  (set `self.bShowMouseCursor` false)
  (`WidgetBlueprintLibrary.SetInputMode_GameOnly` self)
  (`CharacterMovementComponent.SetMovementMode` (`self.GetComponentByClass` (`self.K2_GetPawn`) "/Script/Engine.CharacterMovementComponent") "MOVE_Walking" 0))

(fn `SetInputModeUIOnly `
  (params (InWidgetToFocus :type "Widget Object Reference"))
  (set `self.bShowMouseCursor` true)
  (`WidgetBlueprintLibrary.SetInputMode_UIOnlyEx` self InWidgetToFocus)
  (`CharacterMovementComponent.DisableMovement` (`self.GetComponentByClass` (`self.K2_GetPawn`) "/Script/Engine.CharacterMovementComponent")))

(fn `UserConstructionScript`)